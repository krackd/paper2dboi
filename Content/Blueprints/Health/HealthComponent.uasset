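; HealthComponent is a health component that holds HP and exposes Heal and Damage functions to change it.
; Both functions write HP clamped between zero and MaxHP, and the event graph has no active logic.
; Heal adds Amount to HP, while Damage computes Amount minus HP rather than HP minus Amount, so the subtraction operands are reversed.
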(fn `Damage`
  (params (Amount :type Integer))
  (set `self.HP` (`KismetMathLibrary.Clamp` (- Amount (`self.HP`)) 0 (`self.MaxHP`))))

(fn `Heal`
  (params (Amount :type Integer))
  (set `self.HP` (`KismetMathLibrary.Clamp` (+ Amount (`self.HP`)) 0 (`self.MaxHP`))))